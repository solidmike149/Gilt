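; B_ReloadPoint is a trigger actor that reloads actors that overlap it, then goes on cooldown.
; On overlap, it reads float attributes from the other actor's Ability System Component and, if one is found and below the value it is compared to, tries to activate GA_Reload.
; It then disables BoxComp collision, and a one-shot timer restores query-only collision after Cooldown, whether or not activation succeeded.
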(event Custom|Activate%20Collision
  (Collision|SetCollisionEnabled (Variables|Default|GetBoxComp) "QueryOnly"))

(event Collision|EventActorBeginOverlap
  (params (OtherActor :type Actor%20Object%20Reference))
  (bind _returnvalue (Ability|GetAbilitySystemComponent OtherActor))
  (bind (_bsuccessfullyfoundattribute _returnvalue_2) (Ability|Attribute|GetFloatAttributefromAbilitySystemComponent _returnvalue "(AttributeName=\"Ammo\",Attribute=/Script/ProjectTitan.TiPlayerSet:Ammo,AttributeOwner=None)"))
  (if (and _bsuccessfullyfoundattribute (< _returnvalue_2 (.ReturnValue (Ability|Attribute|GetFloatAttributefromAbilitySystemComponent _returnvalue "(AttributeName=\"MaxAmmo\",Attribute=/Script/ProjectTitan.TiPlayerSet:MaxAmmo,AttributeOwner=None)"))))
    (Abilities|TryActivateAbilitybyClass _returnvalue "/Game/Gilt/Abilities/Player/Reload/GA_Reload.GA_Reload_C" true)
    (Collision|SetCollisionEnabled (Variables|Default|GetBoxComp) "NoCollision")
    (Utilities|Time|SetTimerbyEvent (delegate Custom|Activate%20Collision) (Variables|Default|GetCooldown))))

(fn ConstructionScript)