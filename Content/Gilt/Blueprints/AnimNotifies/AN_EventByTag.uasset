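; AN_EventByTag is an anim notify that sends a gameplay event to the owner of the animated mesh when the animation reaches it.
; The event uses the configured EventTag, and its payload carries a tag container built from PayloadTag.
; The notify's display name in the editor comes from the EventTag name.
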(fn GetNotifyName
  (return (Utilities|String|ToString(Name) (GameplayTags|GetTagName (Variables|Default|GetEvent%20Tag)))))

(fn ReceivedNotify
  (params (MeshComp :type Skeletal%20Mesh%20Component%20Object%20Reference) (Animation :type Anim%20Sequence%20Base%20Object%20Reference) (EventReference :type Anim%20Notify%20Event%20Reference%20Structure%20%28by%20ref%29))
  (Ability|SendGameplayEventtoActor (Components|GetOwner MeshComp) (Variables|Default|GetEvent%20Tag) (Utilities|Struct|MakeGameplayEventData (GameplayTags|MakeGameplayTagContainerfromTag (Variables|Default|GetPayloadTag))))
  (return true))